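; Camera chaser actor that becomes the first player controller's view target on BeginPlay and follows a target actor.
; NewTarget stores a new Target and makes this actor the view target again.
; While the target is valid, Tick lerps location and shortest-path rotation toward it by InterpolationAlpha, a smoothing step that does not scale with delta time.
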(event Custom|NewTarget
  (params (NewTarget :type BP%20Cine%20Camera%20Target%20Object%20Reference))
  (Variables|Default|SetTarget NewTarget)
  (Game|Player|SetViewTargetwithBlend (Game|GetPlayerController 0) self 0.0 "VTBlend_Linear" 0.0 false))

(event EventBeginPlay
  (Game|Player|SetViewTargetwithBlend (Game|GetPlayerController 0) self 0.0 "VTBlend_Linear" 0.0 false))

(event Collision|EventActorBeginOverlap
  (params (OtherActor :type Actor%20Object%20Reference)))

(event EventTick
  (params (DeltaSeconds :type Float%20%28single-precision%29))
  (bind _target (Variables|Default|GetTarget))
  (bind _interpolationalpha (Variables|Default|GetInterpolationAlpha))
  (Utilities|IsValid _target
    (:Is%20Valid
      (Transformation|SetActorLocationAndRotation (Math|Vector|Lerp(Vector) (Transformation|GetActorLocation) (Transformation|GetActorLocation _target) _interpolationalpha) (Math|Rotator|Lerp(Rotator) (Transformation|GetActorRotation) (Transformation|GetActorRotation _target) _interpolationalpha true)))))

(fn ConstructionScript)