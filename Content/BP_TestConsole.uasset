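; BP_TestConsole is a keyboard-driven test harness for controlling a sequence orchestrator and its playback queue.
; Hard-coded key events pause and resume the orchestrator, step to the next or previous sequence, or play queue items 1 and 2 directly.
; Each key calls its orchestrator function and prints the action as feedback, with no other logic in the Blueprint.
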(event EventBeginPlay)

(event Collision|EventActorBeginOverlap
  (params (OtherActor :type Actor%20Object%20Reference)))

(event EventTick
  (params (DeltaSeconds :type Float%20%28single-precision%29)))

(event Input|KeyboardEvents|SpaceBar
  (params (Key :type Key%20Structure :default "None"))
  (:Pressed
    (Class|SequencePlayToolsBPLibrary|PauseOrchestrator)
    (Development|PrintString "Pause")))

(event Input|KeyboardEvents|P
  (params (Key :type Key%20Structure :default "None"))
  (:Pressed
    (Class|SequencePlayToolsBPLibrary|ResumeOrchestrator)
    (Development|PrintString "Resume")))

(event Input|KeyboardEvents|1
  (params (Key :type Key%20Structure :default "None"))
  (:Pressed
    (Class|SequencePlayToolsBPLibrary|PlaySequenceQueueItemat 1)
    (Development|PrintString "Play 1")))

(event Input|KeyboardEvents|2
  (params (Key :type Key%20Structure :default "None"))
  (:Pressed
    (Class|SequencePlayToolsBPLibrary|PlaySequenceQueueItemat 2)
    (Development|PrintString "Play 2")))

(event Input|KeyboardEvents|W
  (params (Key :type Key%20Structure :default "None"))
  (:Pressed
    (Class|SequencePlayToolsBPLibrary|PlayNextSequence)
    (Development|PrintString "Play next")))

(event Input|KeyboardEvents|S
  (params (Key :type Key%20Structure :default "None"))
  (:Pressed
    (Class|SequencePlayToolsBPLibrary|PlayPreviousSequence)
    (Development|PrintString "Play previous")))

(fn ConstructionScript)