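; BP_SequencePlayer is a keyboard-driven trigger that selects and plays one of three items in a sequence queue.
; The number keys 1 to 3 store the matching zero-based index in SequenceToBePlayed, then share one PlaySequenceQueueItemAt call.
; Shift0 to Shift2 inputs only set that index, without starting playback.
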(event Input|KeyboardEvents|Shift0
  (params (Key :type Key%20Structure :default "None"))
  (:Pressed
    (Variables|Default|SetSequenceToBePlayed 0)))

(event Input|KeyboardEvents|Shift1
  (params (Key :type Key%20Structure :default "None"))
  (:Pressed
    (Variables|Default|SetSequenceToBePlayed 1)))

(event Input|KeyboardEvents|Shift2
  (params (Key :type Key%20Structure :default "None"))
  (:Pressed
    (Variables|Default|SetSequenceToBePlayed 2)))

(event Input|KeyboardEvents|1
  (params (Key :type Key%20Structure :default "None"))
  (:Pressed
    (Variables|Default|SetSequenceToBePlayed 0)
    (Class|SequencePlayToolsBPLibrary|PlaySequenceQueueItemat (Variables|Default|GetSequenceToBePlayed))))

(event Input|KeyboardEvents|2
  (params (Key :type Key%20Structure :default "None"))
  (:Pressed
    (Variables|Default|SetSequenceToBePlayed 1)
    (Class|SequencePlayToolsBPLibrary|PlaySequenceQueueItemat (Variables|Default|GetSequenceToBePlayed))))

(event Input|KeyboardEvents|3
  (params (Key :type Key%20Structure :default "None"))
  (:Pressed
    (Variables|Default|SetSequenceToBePlayed 2)
    (Class|SequencePlayToolsBPLibrary|PlaySequenceQueueItemat (Variables|Default|GetSequenceToBePlayed))))

(fn ConstructionScript)